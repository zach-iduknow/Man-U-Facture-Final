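; Inventory component that stores item quantities by name, either in Wood, Metal and Chemical maps or in one General map, depending on SortItemByType.
; ModifyInventory picks the map and calls UpdateInventory, which adds or subtracts, clamps existing stacks to 999 and deletes entries that reach zero.
; For sorted inventories on a player owner, it then notifies BP_AlanController through InventoryUpdated; the General path sends no notification.
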(event `self.ReceiveBeginPlay`)

(fn `Modify Inventory`
  (params (Type :type "/Game/DataSets/ResourceType Enum" :default "NewEnumerator0") (ItemName :type Name) (ItemQuantity :type Integer) (IsRemoving :type Boolean))
  (if (`self.SortItemByType`)
    (switch `/Game/DataSets/ResourceType` Type
      (:`NewEnumerator0`
        (`self.Update Inventory` (`self.WoodInventory`) ItemName ItemQuantity IsRemoving))
      (:`NewEnumerator2`
        (`self.Update Inventory` (`self.MetalInventory`) ItemName ItemQuantity IsRemoving))
      (:`NewEnumerator1`
        (`self.Update Inventory` (`self.ChemicalInventory`) ItemName ItemQuantity IsRemoving)))
    (`/Game/Blueprints/Global/ActorCompMacros.IsPlayerOwner?` null
      (:`Player Owner`
        (bind _asbp_alan_controller (cast `/Game/Blueprints/Alan/BP_AlanController` (`GameplayStatics.GetPlayerController` 0)))
        (`/Game/Blueprints/Alan/BP_AlanController.InventoryUpdated` _asbp_alan_controller Type ItemName)))
    (else
      (`self.Update Inventory` (`self.General`) ItemName ItemQuantity IsRemoving))))

(fn `Update Inventory`
  (params (TargetInventory :type "Map of Name to Integer (by ref)") (ItemName :type "Name (by ref)") (ItemAmount :type Integer) (IsRemoving :type Boolean))
  (locals (Amount :type Integer))
  (bind _returnvalue (`KismetMathLibrary.Clamp` (+ (`BlueprintMapLibrary.Map_Find` TargetInventory ItemName) (`local.Amount`)) 0 999))
  ;[1 1 1] Sets amount to negative if removing an item, keeps it positive if not
  (if IsRemoving
    (set `local.Amount` (* (`KismetMathLibrary.Abs_Int` ItemAmount) -1))
    (else
      (set `local.Amount` (`KismetMathLibrary.Abs_Int` ItemAmount))))
  ;[1 1 1] Checks to see if the target inventory has the item
  (if (`BlueprintMapLibrary.Map_Contains` TargetInventory ItemName)
    (if (> _returnvalue 0)
      ;[1 1 1] Adds item if the amount after removal is greater than 0, removes if it isn't
      (`BlueprintMapLibrary.Map_Add` TargetInventory ItemName _returnvalue)
      (else
        (`BlueprintMapLibrary.Map_Remove` TargetInventory ItemName)))
    (elif (not IsRemoving)
      ;[1 1 1] Adds the item if the inventory doesn't contain it
      (`BlueprintMapLibrary.Map_Add` TargetInventory ItemName (`local.Amount`)))))