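; BP_HealthComponent is a health component that tracks a Health value against a MaxHealth limit.
; Health starts at MaxHealth on BeginPlay, and TakeDamage subtracts positive damage, clamps the result between zero and MaxHealth, and returns it.
; IsActorAlive reports whether Health is above zero; the component itself fires no death or change events and does no Tick work.
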(event `self.ReceiveBeginPlay`
  (set `self.Health` (`self.MaxHealth`)))

(fn `IsActorAlive?`
  (returns (Result :type Boolean))
  (return (> (`self.Health`) 0.0)))

(fn `TakeDamage`
  (params (Damage :type "Float (double-precision)"))
  (returns (HealthRemaining :type "Float (double-precision)"))
  (if (> Damage 0.0)
    (bind _output_get (set `self.Health` (`KismetMathLibrary.FClamp` (- (`self.Health`) Damage) 0.0 (`self.MaxHealth`))))
    (return _output_get)))