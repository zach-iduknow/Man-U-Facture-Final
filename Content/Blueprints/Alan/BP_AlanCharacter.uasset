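; Alan, the click-to-move player character, who harvests resources and uses factories.
; A click paths him to the cursor hit and stores the clicked actor, while Tick smoothly turns control rotation toward the target.
; Overlapping that actor with ResourceDetection opens a factory or starts a delayed damage loop on wood, the only resource type handled.
; Damage goes to the controller's Health; death destroys the pawn, which saves its location to the controller.
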(event `self.ReceiveBeginPlay`
  ;[1 1 1] Component Variable Setup
  (bind _asbp_alan_controller (cast `/Game/Blueprints/Alan/BP_AlanController` (`GameplayStatics.GetPlayerController` 0)))
  (set `self.AlanController` _asbp_alan_controller))

(event `InputAction|ClickMove`
  (params (Key :type "Key Structure"))
  ;[0 0.5115 0.9323] Movement
  (:`Pressed`
    (`self.MoveAndScan`)))

(event `self.ReceiveAnyDamage`
  (params (Damage :type "Float (single-precision)") (DamageType :type "DamageType Object Reference") (InstigatedBy :type "Controller Object Reference") (DamageCauser :type "Actor Object Reference"))
  (bind _health (`/Game/Blueprints/Alan/BP_AlanController.Health` (`self.AlanController`)))
  ;[1 0.1198 0.1198] Logic For Taking Damage
  (bind _healthremaining (`/Game/Blueprints/Components/BP_HealthComponent.TakeDamage` _health Damage))
  (`KismetSystemLibrary.PrintString` (`KismetStringLibrary.Conv_DoubleToString` _healthremaining))
  (`/Game/Blueprints/Global/GlobalMacros.IsAlive?` _health
    (:`Dead`
      (`self.KillPlayer`))))

(event `self.ReceiveTick`
  (params (DeltaSeconds :type "Float (single-precision)"))
  ;[0.3122 1 0.371] Tick functions for turning the player
  (`self.TurnToLocation`))

(event `self.ReceiveDestroyed`
  (`/Game/Blueprints/Alan/BP_AlanController.SetAlanLocation` (`self.AlanController`) (`self.K2_GetActorLocation`)))

(event `self.Resource Detection.OnComponentBeginOverlap`
  (params (OverlappedComponent :type "PrimitiveComponent Object Reference") (OtherActor :type "Actor Object Reference") (OtherComp :type "PrimitiveComponent Object Reference") (OtherBodyIndex :type Integer) (bFromSweep :type Boolean) (SweepResult :type "HitResult Structure (by ref)"))
  (bind _clickedactor (`self.ClickedActor`))
  (if (== OtherActor _clickedactor)
    (bind _asbp_level_resource (cast `/Game/Blueprints/Resources/BP_LevelResource` _clickedactor)
      (:`then`
        (`MovementComponent.StopMovementImmediately` (`self.CharacterMovement`))
        (switch `/Game/DataSets/ResourceType` (`/Game/Blueprints/Resources/BP_LevelResource.ResourceType` _asbp_level_resource)
          (:`NewEnumerator0`
            (bind _output_get (set `self.Chopping` true))
            (`self.StartHarvest` _asbp_level_resource (`self.ChopDamage`) (`self.ChopTime`) _output_get))))
      (:`CastFailed`
        (bind _asbp_factory (cast `/Game/Blueprints/Buildings/BP_Factory` _clickedactor)
          (:`then`
            (`KismetSystemLibrary.PrintString` "I'm at a factory!")
            (`MovementComponent.StopMovementImmediately` (`self.CharacterMovement`))
            (`/Game/Blueprints/Alan/BP_AlanController.OpenFactory` (`self.AlanController`) _asbp_factory))
          (:`CastFailed`
            (`KismetSystemLibrary.PrintString` "Can't interact!")))))))

(fn `KillPlayer`
  (`self.DetachFromControllerPendingDestroy`)
  (`self.K2_DestroyActor`))

(fn `MoveAndScan`
  (bind (_bblockinghit _binitialoverlap _time _distance _location _impactpoint _normal _impactnormal _physmat _hitactor) (`GameplayStatics.BreakHitResult` (`PlayerController.GetHitResultUnderCursorByChannel` (`self.AlanController`) "TraceTypeQuery1" true)))
  (bind (_returnvalue_roll _returnvalue_pitch _returnvalue_yaw) (`KismetMathLibrary.BreakRotator` (`KismetMathLibrary.FindLookAtRotation` (`SceneComponent.K2_GetComponentLocation` (`self.CapsuleComponent`)) _location)))
  (`/Game/Blueprints/Alan/BP_AlanController.CloseFactory` (`self.AlanController`))
  (`self.ResetHarvestState`)
  (`AIBlueprintHelperLibrary.SimpleMoveToLocation` (`self.AlanController`) _location)
  (set `self.ClickedActor` _hitactor)
  (set `self.TargetRotation` (`KismetMathLibrary.MakeRotator` 0.0 0.0 _returnvalue_yaw)))

(fn `ResetHarvestState`
  (set `self.Chopping` false)
  (set `self.Mining` false)
  (set `self.Vacuuming` false))

(fn `SetAlanDisable`
  (params (Disable :type Boolean))
  (if Disable
    (`SceneComponent.SetVisibility` (`self.Mesh`) false false)
    (`PrimitiveComponent.SetCollisionObjectType` (`self.CapsuleComponent`) "ECC_WorldStatic")
    (else
      (`SceneComponent.SetVisibility` (`self.Mesh`) true false)
      (`PrimitiveComponent.SetCollisionObjectType` (`self.CapsuleComponent`) "ECC_Pawn"))))

(fn `TurnToLocation`
  (bind _returnvalue (`Controller.GetControlRotation` (`self.AlanController`)))
  (if (!= (`self.TargetRotation`) _returnvalue)
    (`Controller.SetControlRotation` (`self.AlanController`) (`KismetMathLibrary.RInterpTo` _returnvalue (`self.TargetRotation`) (`GameplayStatics.GetWorldDeltaSeconds`) (`self.TurnSpeed`)))))

(fn `UserConstructionScript`)