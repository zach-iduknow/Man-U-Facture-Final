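; BP_LevelResource is a damageable resource actor that breaks into item drops when its health runs out.
; AnyDamage passes damage to the Health component, then checks whether it is dead.
; On death, it spawns a random number of ItemToDrop actors at its mesh location, then destroys itself.
; Each drop's mesh gets a mass-independent impulse, randomized per axis within plus or minus DropRange, to scatter the items.
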(event `self.ReceiveAnyDamage`
  (params (Damage :type "Float (single-precision)") (DamageType :type "DamageType Object Reference") (InstigatedBy :type "Controller Object Reference") (DamageCauser :type "Actor Object Reference"))
  (bind _health (`self.Health`))
  (`/Game/Blueprints/Components/BP_HealthComponent.TakeDamage` _health Damage)
  (`/Game/Blueprints/Global/GlobalMacros.IsAlive?` _health
    (:`Dead`
      (for _ (range (+ (`KismetMathLibrary.RandomIntegerInRange` (`self.ItemDropMin`) (`self.ItemDropMax`)) 1))
        (bind _returnvalue (`|SpawnActorFromClass` (`self.ItemToDrop`) (`KismetMathLibrary.MakeTransform` (`SceneComponent.K2_GetComponentLocation` (`self.StaticMesh`))) "Undefined" "OverrideRootScale" null null))
        (`PrimitiveComponent.AddImpulse` (`/Game/Blueprints/Resources/BP_PickUp.StaticMesh` _returnvalue) (`self.GetRandomDirection`) "None" true))
      (`self.K2_DestroyActor`))))

(fn `GetRandomDirection`
  (returns (ReturnValue :type "Vector Structure"))
  (bind _droprange (`self.DropRange`))
  (bind _returnvalue (* _droprange -1.0))
  (return (`KismetMathLibrary.MakeVector` (`KismetMathLibrary.RandomFloatInRange` _returnvalue _droprange) (`KismetMathLibrary.RandomFloatInRange` _returnvalue _droprange) (`KismetMathLibrary.RandomFloatInRange` _returnvalue _droprange))))

(fn `UserConstructionScript`)