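; Base building actor for a survival game: a ghost preview that becomes a solid, placed structure.
; While in ghost state, Tick grid-snaps the box's current location and swaps valid/invalid materials based on tracked overlapping blockers; cancel destroys it.
; Outside that state, Tick calls PlaceBuilding every frame to check and remove inventory items, then enable blocking collision.
; PlayerHasItem is a stub returning false, and placement never checks blockers.
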(event `self.ReceiveTick`
  (params (DeltaSeconds :type "Float (single-precision)"))
  (if (`|EnumEquality` (`self.BuildingState`) "NewEnumerator0")
    (`self.IsLocationValid?`)
    (`self.FollowMouse`)
    (else
      (`self.Place Building`)
      (`KismetSystemLibrary.PrintString` "Building placed!"))))

(event `self.ReceiveBeginPlay`
  (`self.BuildingSetup`))

(event `InputAction|CancelBuild`
  (params (Key :type "Key Structure"))
  ;[0.849 0 0.04084] Logic for destroying the building on cancel
  (:`Pressed`
    (if (`|EnumEquality` (`self.BuildingState`) "NewEnumerator0")
      (`self.K2_DestroyActor`))))

(event `self.Box.OnComponentBeginOverlap`
  (params (OverlappedComponent :type "PrimitiveComponent Object Reference") (OtherActor :type "Actor Object Reference") (OtherComp :type "PrimitiveComponent Object Reference") (OtherBodyIndex :type Integer) (bFromSweep :type Boolean) (SweepResult :type "HitResult Structure (by ref)"))
  ;[1 1 1] Adds and removes overlapping obejcts to building blocker
  (`KismetArrayLibrary.Array_Add` (`self.BuildingBlockers`) OtherActor))

(event `self.Box.OnComponentEndOverlap`
  (params (OverlappedComponent :type "PrimitiveComponent Object Reference") (OtherActor :type "Actor Object Reference") (OtherComp :type "PrimitiveComponent Object Reference") (OtherBodyIndex :type Integer))
  ;[1 1 1] Adds and removes overlapping obejcts to building blocker
  (`KismetArrayLibrary.Array_RemoveItem` (`self.BuildingBlockers`) OtherActor))

(fn `BuildingSetup`
  (bind _box (`self.Box`))
  (`PrimitiveComponent.SetMaterial` (`self.Mesh`) 0 "/Game/Meshes/Materials/MI_BuildGhostValid.MI_BuildGhostValid")
  (`PrimitiveComponent.SetMaterial` (`self.AnimMesh`) 0 "/Game/Meshes/Materials/MI_BuildGhostValid.MI_BuildGhostValid")
  (bind _asbp_alan_controller (cast `/Game/Blueprints/Alan/BP_AlanController` (`GameplayStatics.GetPlayerController` 0))
    (:`then`
      (set `self.AlanController` _asbp_alan_controller)
      (bind _asgm_survival (cast `/Game/Blueprints/GameModes/GM_Survival` (`GameplayStatics.GetGameMode`))
        (:`then`
          (set `self.ActiveGamemode` _asgm_survival)
          (`PrimitiveComponent.SetCollisionEnabled` _box "QueryOnly")
          (`PrimitiveComponent.SetCollisionResponseToAllChannels` _box "ECR_Ignore")
          (`PrimitiveComponent.SetCollisionResponseToChannel` _box "ECC_GameTraceChannel2" "ECR_Overlap")
          (`PrimitiveComponent.SetCollisionResponseToChannel` _box "ECC_GameTraceChannel1" "ECR_Overlap")
          (`PrimitiveComponent.SetCollisionResponseToChannel` _box "ECC_GameTraceChannel3" "ECR_Overlap")
          (`PrimitiveComponent.SetCollisionResponseToChannel` _box "ECC_Pawn" "ECR_Overlap"))
        (:`CastFailed`
          (`KismetSystemLibrary.PrintString` "Building couldn't find game mode!" true true (struct :`R` 0.848958 :`B` 0.040841 :`A` 1.0)))))
    (:`CastFailed`
      (`KismetSystemLibrary.PrintString` "Building couldn't find controller!" true true (struct :`R` 0.848958 :`B` 0.040841 :`A` 1.0)))))

(fn `FollowMouse`
  (bind (_returnvalue_x _returnvalue_y _returnvalue_z) (`KismetMathLibrary.BreakVector` (`SceneComponent.K2_GetComponentLocation` (`self.Box`))))
  (bind _returnvalue (`KismetMathLibrary.Conv_IntToDouble` (`/Game/Blueprints/GameModes/GM_Survival.GridBuildSize` (`self.ActiveGamemode`))))
  (`SceneComponent.K2_SetWorldLocation` (`self.Box`) (`KismetMathLibrary.MakeVector` (`KismetMathLibrary.GridSnap_Float` _returnvalue_x _returnvalue) (`KismetMathLibrary.GridSnap_Float` _returnvalue_y _returnvalue) _returnvalue_z) false true))

(fn `IsLocationValid?`
  (if (`KismetArrayLibrary.Array_IsEmpty` (`self.BuildingBlockers`))
    (`self.SetBuildingMaterial` (`self.ValidGhostMat`))
    (else
      (`self.SetBuildingMaterial` (`self.InvalidGhostMat`)))))

(fn `Place Building`
  (bind _box (`self.Box`))
  ;[0.849 0 0.04084] Iterates over required items to see if player has them, returns out of the function if they don't
  (bind (_array_element _value) (`/Game/Blueprints/Global/GlobalMacros.IterateMap` (`self.ItemsNeeded`))
    (:`LoopBody`
      (bind _result (`self.PlayerHasItem` _array_element _value))
      (if (not _result)
        (`KismetSystemLibrary.PrintString` "Not enough items!")
        (return)))
    (:`Completed`
      ;[0.6771 0.5734 0.2432] Iterates through required items again, this time it removes the item
      (bind (_array_element_2 _value_2) (`/Game/Blueprints/Global/GlobalMacros.IterateMap` (`self.ItemsNeeded`))
        (:`LoopBody`
          (bind _returnvalue (`|GetDataTableRow` "/Game/DataSets/ResourceTable.ResourceTable" _array_element_2)
            (:`then`
              (`/Game/Blueprints/Components/BP_InventoryComponent.Modify Inventory` (`/Game/Blueprints/Alan/BP_AlanController.Inventory` (`self.AlanController`)) (`.ItemType_5_315A3BAD426286D67749A1BE601CFC29` (break `/Game/DataSets/Resource` _returnvalue)) _array_element_2 _value_2 true))))
        (:`Completed`
          ;[0.1087 1 0.3386] Places building by switching the state to placed, setting the material on the active mesh, and turning on collisions
          (set `self.BuildingState` "NewEnumerator1")
          (`self.SetBuildingMaterial` (`self.PlacedMat`))
          (`PrimitiveComponent.SetCollisionEnabled` _box "QueryAndPhysics")
          (`PrimitiveComponent.SetCollisionResponseToAllChannels` _box "ECR_Block"))))))

(fn `PlayerHasItem`
  (params (ItemName :type Name) (ItemAmount :type Integer))
  (returns (Result :type Boolean))
  (return false))

(fn `SetBuildingMaterial`
  (params (Material :type "MaterialInterface Object Reference"))
  (bind _animmesh (`self.AnimMesh`))
  (bind _mesh (`self.Mesh`))
  (`/Engine/EditorBlueprintResources/StandardMacros.IsValid` _animmesh
    (:`Is Valid`
      (`PrimitiveComponent.SetMaterial` _animmesh 0 Material))
    (:`Is Not Valid`
      (`/Engine/EditorBlueprintResources/StandardMacros.IsValid` _mesh
        (:`Is Valid`
          (`PrimitiveComponent.SetMaterial` _mesh 0 Material))))))

(fn `UserConstructionScript`)