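; Factory building that crafts furniture from three chosen items, spawning pieces one at a time.
; CraftingStarted stores the items, sets the repeat count to the smallest supplied amount and starts a looping timer on CraftFurniture.
; Each tick of that timer spawns the target furniture, applies the items' materials and launches it against the spawn point's forward vector.
; The timer clears when CraftCount reaches the repeat count; the counter is never reset here.
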(event `CraftingStarted`
  (params (PrimaryItem :type Name) (PrimAmount :type Integer) (SecondaryItem :type Name) (SecAmount :type Integer) (TertiaryItem :type Name) (TertAmount :type Integer))
  ;[1 1 1] Setting the item values here was an alternative to timer delegates :/
  (set `self.Primary Item` PrimaryItem)
  (set `self.Secondary Item` SecondaryItem)
  (set `self.Tertiary Item` TertiaryItem)
  (set `self.CraftReps` (`KismetMathLibrary.Min` PrimAmount SecAmount TertAmount))
  (bind _returnvalue (`KismetSystemLibrary.K2_SetTimer` null "CraftFurniture" (`self.CraftTime`) true))
  (set `self.CraftTimerHandle` _returnvalue))

(fn `CraftFurniture`
  (bind _returnvalue (`|SpawnActorFromClass` (`self.TargetFurniture`) (`KismetMathLibrary.MakeTransform` (`SceneComponent.K2_GetComponentLocation` (`self.FurnitureSpawn`))) "Undefined" "OverrideRootScale" null null))
  (bind _item_material (`/Game/Blueprints/Global/GlobalMacros.GetItemMaterial` (`self.Primary Item`)))
  (bind _item_material_2 (`/Game/Blueprints/Global/GlobalMacros.GetItemMaterial` (`self.Secondary Item`)))
  (bind _item_material_3 (`/Game/Blueprints/Global/GlobalMacros.GetItemMaterial` (`self.Tertiary Item`)))
  (`/Game/Blueprints/Furniture/BP_Furniture.AssignAttributes` _returnvalue _item_material _item_material_2 _item_material_3)
  (`PrimitiveComponent.AddImpulse` (`/Game/Blueprints/Furniture/BP_Furniture.Box` _returnvalue) (* (`SceneComponent.GetForwardVector` (`self.FurnitureSpawn`)) -500.0) "None" true)
  (bind _result (`/Engine/EditorBlueprintResources/StandardMacros.IncrementInt` (`self.CraftCount`))
    (:`  `
      (if (< _result (`self.CraftReps`))
        (return)
        (else
          (`KismetSystemLibrary.K2_ClearAndInvalidateTimerHandle` (`self.CraftTimerHandle`))
          (`KismetSystemLibrary.PrintString` "Crafting Complete!" true true (struct :`R` 0.677083 :`G` 0.161973 :`B` 0.094456 :`A` 1.0)))))))

(fn `UserConstructionScript`
  (`parent.UserConstructionScript`))